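; BP_GameShowPlayerData is a game show player data Blueprint that expects a PlayerState as its owner and supplies an identifier for that player.
; GetEffectiveIdentifier returns the stored PlayerIdentifier, falling back to the owning PlayerState's player name when it is empty.
; If the owner is not a PlayerState, it logs an error and returns the stored value.
; BeginPlay only logs the spawn and whether it runs on server or client.
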(event `self.ReceiveBeginPlay`
  (`BlueprintLoggingLibrary.LogVerbose` (`KismetStringLibrary.Concat_StrStr` (`KismetSystemLibrary.GetDisplayName` self) " Spawned"))
  (`/Engine/EditorBlueprintResources/ActorComponentMacros.Switch Has Authority`
    (:`Authority`
      (`BlueprintLoggingLibrary.LogVerbose` "Server side"))
    (:`Remote`
      (`BlueprintLoggingLibrary.LogVerbose` "Client side"))))

(fn `Get Effective Identifier`
  (returns (`Player Identifier` :type String))
  (bind _playeridentifier (`self.PlayerIdentifier`))
  (bind _asplayer_state (cast `PlayerState` (`self.GetOwner`))
    (:`then`
      (return (`KismetMathLibrary.SelectString` (`PlayerState.GetPlayerName` _asplayer_state) _playeridentifier (`KismetStringLibrary.IsEmpty` _playeridentifier))))
    (:`CastFailed`
      (`BlueprintLoggingLibrary.LogError` "Owner was not PlayerState")
      (return _playeridentifier))))